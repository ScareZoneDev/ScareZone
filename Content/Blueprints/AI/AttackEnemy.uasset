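; Behavior tree task that makes an AI character attack the VR player once in range.
; The first tick caches the controller and pawn; later ticks read the target from the blackboard.
; A short multi-sphere trace around the AI, ignoring all AI characters, confirms the hit before triggering the attack and finishing successfully.
; An invalid target fails the task, while an out-of-range one leaves it running.
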(event EventTick
  (params (OwnerActor :type Actor%20Object%20Reference) (DeltaSeconds :type Float%20%28single-precision%29))
  ;[1 1 1] confirm hit
  (if (== (Variables|Default|GetAIController) 0)
    (bind _asbasic_aicontroller (Utilities|Casting|CastToBasicAIController OwnerActor)
      (:then
        (bind _output_get (Variables|Default|SetAIController _asbasic_aicontroller))
        (bind _asaicharacter (Utilities|Casting|CastToAICharacter (Pawn|GetControlledPawn _output_get))
          (:then
            (Variables|Default|SetAICharacter _asaicharacter))
          (:CastFailed
            (Development|PrintString "CAST FAILED"))))
      (:CastFailed
        (Development|PrintString "ERROR CASTING")))
    (else
      (bind _asvrfirst_person_character (Utilities|Casting|CastToVRFirstPersonCharacter (Class|BTFunctionLibrary|GetBlackboardValueasObject (Variables|Default|GetEnemyToAttack)))
        (:then
          (Variables|Default|SetEnemy _asvrfirst_person_character)
          (bind _outactors (Actor|GetAllActorsOfClass "/Game/Blueprints/AI/AICharacter.AICharacter_C"))
          (bind _outhits (Collision|MultiSphereTraceForObjects (Transformation|GetActorLocation (Variables|Default|GetAICharacter)) (+ (Transformation|GetActorLocation (Variables|Default|GetAICharacter)) "0, 0,15.000000") 2e+02 (Variables|Default|GetDesiredObjectTypes) false _outactors "None"))
          (bind _array_element (Utilities|Array|ForEachLoopwithBreak _outhits)
            (:LoopBody
              (if (== (.HitActor (Collision|BreakHitResult _array_element)) (Variables|Default|GetEnemy))
                (Default|EventAttack (Variables|Default|GetAICharacter) (Variables|Default|GetEnemy))
                (AI|BehaviorTree|FinishExecute true)))))
        (:CastFailed
          (AI|BehaviorTree|FinishExecute false))))))