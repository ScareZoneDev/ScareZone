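; AI character Blueprint for an enemy that runs a behavior tree and damages the player when attacking.
; On BeginPlay it stores its spawn location and starts the tree on its AI controller.
; Attack deals damage through a Gate that closes during a timed attacking flag and reopens after an attack-speed cooldown.
; Tick switches max walk speed between engaged and idle values.
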(event Custom|Event%20Attack
  (params (Enemy :type VR%20First%20Person%20Character%20Object%20Reference))
  (Utilities|FlowControl|Gate false :!label _label
    (:Exit
      (Variables|Default|SetAttacking? true)
      (Default|DamagePlayer Enemy (Variables|AI|GetDamageModifier))
      (Utilities|FlowControl|Sequence
        (:then_0
          (goto _label Close))
        (:then_1
          (Utilities|FlowControl|Delay 1.5)
          (Variables|Default|SetAttacking? false)
          (Utilities|FlowControl|Delay (Variables|AI|GetAttackSpeed))
          (goto _label Open))))))

(event EventBeginPlay
  ;[1 1 1] Set Spawn
  (Variables|Default|SetSpawnLocation (Transformation|GetActorLocation))
  (bind _returnvalue (AI|GetAIController self))
  (AI|RunBehaviorTree _returnvalue (Variables|Default|GetAIBehaviorTree)))

(event EventActorBeginOverlap
  (params (OtherActor :type Actor%20Object%20Reference)))

(event EventTick
  (params (DeltaSeconds :type Float%20%28single-precision%29))
  (bind _charactermovement (Variables|Character|GetCharacterMovement))
  (if (Variables|AI|GetisEngaged)
    (Variables|/Script/Engine.CharacterMovementComponent|SetMaxWalkSpeed _charactermovement (Variables|Default|GetMaxSpeed_Engaged))
    (else
      (Variables|/Script/Engine.CharacterMovementComponent|SetMaxWalkSpeed _charactermovement (Variables|Default|GetMaxSpeed_Idle)))))

(fn ConstructionScript)