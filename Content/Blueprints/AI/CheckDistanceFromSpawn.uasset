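; Behavior tree node that leashes an AI by dropping its follow target when that target strays too far from the AI's spawn point.
; Each tick it casts the owner to BasicAIController and its pawn to AICharacter, then measures from SpawnLocation to the TargetToFollow actor, not the pawn.
; Beyond MaxKiteDistance it clears that blackboard key.
; It prints the distance and any cast failures for debugging, and never validity-checks the target.
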(event EventTick
  (params (OwnerActor :type Actor%20Object%20Reference) (DeltaSeconds :type Float%20%28single-precision%29))
  (Utilities|IsValid OwnerActor
    (:Is%20Valid
      (bind _asbasic_aicontroller (Utilities|Casting|CastToBasicAIController OwnerActor)
        (:then
          (bind _output_get (Variables|Default|SetAIController _asbasic_aicontroller))
          (bind _asaicharacter (Utilities|Casting|CastToAICharacter (Pawn|GetControlledPawn _output_get))
            (:then
              (Development|PrintString (Utilities|String|ToString(Float) (Math|Vector|VectorLength (- (Transformation|GetActorLocation (AI|BehaviorTree|GetBlackboardValueasActor (Variables|Default|GetTargetToFollow))) (Variables|/Game/Blueprints/AI/AICharacter.AICharacter_C|GetSpawnLocation _asaicharacter)))))
              (if (> (Math|Vector|VectorLength (- (Transformation|GetActorLocation (AI|BehaviorTree|GetBlackboardValueasActor (Variables|Default|GetTargetToFollow))) (Variables|/Game/Blueprints/AI/AICharacter.AICharacter_C|GetSpawnLocation _asaicharacter))) (Variables|/Game/Blueprints/AI/AICharacter.AICharacter_C|GetMaxKiteDistance _asaicharacter))
                (Class|BTFunctionLibrary|SetBlackboardValueasObject (Variables|Default|GetTargetToFollow))))
            (:CastFailed
              (Development|PrintString "CAST TO AICHARACTER FAILED" true true "(R=1.000000,G=0.000000,B=0.000000,A=1.000000)"))))
        (:CastFailed
          (Development|PrintString "CAST TO AICONTROLLER FAILED" true true "(R=1.000000,G=0.000000,B=0.000000,A=1.000000)"))))))