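; Behavior tree node that makes an AICharacter follow the VR player except when watched, judged by overlap and line of sight.
; Each tick it caches controller and pawn, then, once cached, sets TargetToFollow to the player.
; An AgroRange sphere trace, meant as a range check, clears the key on any non-player hit, but not on zero hits.
; Player overlap plus an unblocked camera-channel trace also clears it.
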(event EventTick
  (params (OwnerActor :type Actor%20Object%20Reference) (DeltaSeconds :type Float%20%28single-precision%29))
  (if (== (Variables|Default|GetAIController) 0)
    (bind _asaicontroller (Utilities|Casting|CastToAIController OwnerActor))
    (bind _output_get (Variables|Default|SetAIController _asaicontroller))
    (bind _asaicharacter (Utilities|Casting|CastToAICharacter (Pawn|GetControlledPawn _output_get)))
    (Variables|Default|SetAICharacter _asaicharacter)
    (else
      (Variables|Default|SetMyLocation (Transformation|GetActorLocation (Variables|Default|GetAICharacter)))
      (bind _asvrfirst_person_character (Utilities|Casting|CastToVRFirstPersonCharacter (Game|GetPlayerCharacter 0)))
      (Variables|Default|SetFirstPersonCharacter _asvrfirst_person_character)
      (Class|BTFunctionLibrary|SetBlackboardValueasObject (Variables|Default|GetTargetToFollow) (Variables|Default|GetFirstPersonCharacter))
      (Utilities|FlowControl|Sequence
        (:then_0
          ;[1 1 1] Range Check
          (bind _outactors (Actor|GetAllActorsOfClass "/Game/Blueprints/AI/AICharacter.AICharacter_C"))
          (bind _outhits (Collision|MultiSphereTraceForObjects (Variables|Default|GetMyLocation) (+ (Variables|Default|GetMyLocation) "0, 0,15.000000") (Variables|/Game/Blueprints/AI/AICharacter.AICharacter_C|GetAgroRange (Variables|Default|GetAICharacter)) (Variables|Default|GetDesiredObjectTypes) false _outactors "None"))
          (bind _array_element (Utilities|Array|ForEachLoopwithBreak _outhits)
            (:LoopBody
              ;;[1 1 1] Clear Target to Follow if player is out of Range
              (if (not (== (Variables|Default|GetFirstPersonCharacter) (.HitActor (Collision|BreakHitResult _array_element))))
                (Class|BTFunctionLibrary|SetBlackboardValueasObject (Variables|Default|GetTargetToFollow))))))
        (:then_1
          ;[1 1 1] Check if this AI is in the player's vision cone
          (if (Collision|IsOverlappingActor (Variables|Default|GetAICharacter) (Variables|Default|GetFirstPersonCharacter) :!class /Script/Engine.Actor)
            ;[1 1 1] Ray trace from player to AI to confirm hit
            (bind _outactors_2 (Actor|GetAllActorsOfClass "/Game/Blueprints/AI/AICharacter.AICharacter_C"))
            (bind _outhit (Collision|LineTraceByChannel (Variables|Default|GetMyLocation) (Transformation|GetActorLocation (Variables|Default|GetFirstPersonCharacter)) "TraceTypeQuery2" false _outactors_2 "None"))
            ;;[1 1 1] Clear Target to Follow if Player is "Watching" AI
            (if (== (.HitActor (Collision|BreakHitResult _outhit)) (Variables|Default|GetFirstPersonCharacter))
              (Class|BTFunctionLibrary|SetBlackboardValueasObject (Variables|Default|GetTargetToFollow)))))))))