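; AgroCheck is a ticking behavior tree node that detects targets for an AICharacter and engages it.
; It caches the controller and pawn, then sphere-traces at the controller's location using AgroRange and the desired object types, ignoring all AICharacters.
; A Camera-channel line trace checks sight to each hit.
; Visible actors are written to the TargetToFollow blackboard key, and the pawn's IsEngaged flag is set.
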(event EventTick
  (params (OwnerActor :type Actor%20Object%20Reference) (DeltaSeconds :type Float%20%28single-precision%29))
  (if (== (Variables|Default|GetAIController) 0)
    (bind _asbasic_aicontroller (Utilities|Casting|CastToBasicAIController OwnerActor))
    (bind _output_get (Variables|Default|SetAIController _asbasic_aicontroller))
    (bind _asaicharacter (Utilities|Casting|CastToAICharacter (Pawn|GetControlledPawn _output_get)))
    (Variables|Default|SetAICharacter _asaicharacter)
    (else
      (bind _outactors (Actor|GetAllActorsOfClass "/Game/Blueprints/AI/AICharacter.AICharacter_C"))
      (Variables|Default|SetMyLocation (Transformation|GetActorLocation (Variables|Default|GetAIController)))
      (bind _outhits (Collision|MultiSphereTraceForObjects (Transformation|GetActorLocation (Variables|Default|GetAIController)) (+ (Transformation|GetActorLocation (Variables|Default|GetAIController)) "0, 0,15.000000") (Variables|/Game/Blueprints/AI/AICharacter.AICharacter_C|GetAgroRange (Variables|Default|GetAICharacter)) (Variables|Default|GetDesiredObjectTypes) false _outactors "ForDuration"))
      (bind _array_element (Utilities|Array|ForEachLoopwithBreak _outhits)
        (:LoopBody
          (bind _outhit (Collision|LineTraceByChannel (Variables|Default|GetMyLocation) (Transformation|GetActorLocation (.HitActor (Collision|BreakHitResult _array_element))) "TraceTypeQuery2" false _outactors "None"))
          (if (== (.HitActor (Collision|BreakHitResult _outhit)) (.HitActor (Collision|BreakHitResult _array_element)))
            (Class|BTFunctionLibrary|SetBlackboardValueasObject (Variables|Default|GetTargetToFollow) (.HitActor (Collision|BreakHitResult _outhit)))
            (bind _asaicharacter_2 (Utilities|Casting|CastToAICharacter (Pawn|GetControlledPawn (Variables|Default|GetAIController))))
            (Variables|/Game/Blueprints/AI/AICharacter.AICharacter_C|SetisEngaged _asaicharacter_2 true)))))))